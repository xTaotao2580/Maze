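; BP_Étoile is a star actor that ends the game when the player character overlaps it.
; It caches BP_ThirdPersonGameMode on BeginPlay and calls its FinDuJeu on that overlap.
; The same overlap prints a debug string, plays the Windows XP startup sound at the world origin, and eases the star mesh upward with a rotation before destroying the actor.
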(event `self.ReceiveBeginPlay`
  (bind _asbp_third_person_game_mode (cast `/Game/Blueprints/BP_ThirdPersonGameMode` (`GameplayStatics.GetGameMode`)))
  (set `self.REF gamemode` _asbp_third_person_game_mode))

(event `self.ReceiveActorBeginOverlap`
  (params (OtherActor :type "Actor Object Reference"))
  (if (== OtherActor (`GameplayStatics.GetPlayerCharacter` 0))
    (`|ExecutionSequence`
      (:`then_0`
        (`/Game/Blueprints/BP_ThirdPersonGameMode.Fin du jeu` (`self.REF gamemode`)))
      (:`then_1`
        (`KismetSystemLibrary.PrintString` "Playing sound")
        (`GameplayStatics.PlaySoundAtLocation` "/Game/Assets/Sound/Microsoft_Windows_XP_Startup_Sound_01.Microsoft_Windows_XP_Startup_Sound_01" (0.0 0.0 0.0) (struct) 1.0 1.0 0.0 null null null))
      (:`then_2`
        (`KismetSystemLibrary.MoveComponentTo` (`self.Étoile_mesh`) (0.0 0.0 2000.0) (struct :`Pitch` 45.0 :`Yaw` 45.0 :`Roll` 45.0) false true 2.5 true)
        (`self.K2_DestroyActor`)))))

(fn `UserConstructionScript`)