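; BP_Porte is a door actor that slides open when its Ouverture_Porte event is called.
; The construction script sets its point light to red, and the event switches it to green.
; The event then plays a timeline that lerps the door component's relative location from StartLoc to EndLoc.
; No closing logic is present, and nothing in this Blueprint itself triggers the opening.
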(event `Ouverture_Porte`
  (`LightComponent.SetLightColor` (`self.PointLight`) (struct :`G` 1.0 :`B` 0.041276 :`A` 1.0) true)
  (bind (_direction _newtrack_0) (`Timeline|Timeline_0`)
    (:`Update`
      (`SceneComponent.K2_SetRelativeLocation` (`self.Porte`) (`KismetMathLibrary.VLerp` (`self.Start Loc`) (`self.End Loc`) _newtrack_0) false false))))

(fn `UserConstructionScript`
  (`LightComponent.SetLightColor` (`self.PointLight`) (struct :`R` 1.0 :`A` 1.0) true))