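; BP_Levier is a one-shot lever the player activates with the Activer action while in range.
; Box overlaps enable or disable its input and show or hide the player character's BoutonE prompt, without checking which actor overlapped.
; The construction script tints CubeLevier through a dynamic material using Couleur.
; The first press turns it red and prints "+1"; a DoOnce blocks further presses.
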(event `InputAction|Activer`
  (params (Key :type "Key Structure"))
  (:`Pressed`
    (`/Engine/EditorBlueprintResources/StandardMacros.DoOnce` false
      (:`Completed`
        (`KismetSystemLibrary.PrintString` "+1")
        (`MaterialInstanceDynamic.SetVectorParameterValue` (`self.M_DynLevier`) "Color" (struct :`R` 1.0 :`G` 0.018362 :`A` 1.0))))))

(event `self.Box.OnComponentBeginOverlap`
  (params (OverlappedComponent :type "PrimitiveComponent Object Reference") (OtherActor :type "Actor Object Reference") (OtherComp :type "PrimitiveComponent Object Reference") (OtherBodyIndex :type Integer) (bFromSweep :type Boolean) (SweepResult :type "HitResult Structure (by ref)"))
  (`self.EnableInput` (`GameplayStatics.GetPlayerController` 0))
  (bind _asthird_person_character (cast `/Game/ThirdPersonBP/Blueprints/ThirdPersonCharacter` (`GameplayStatics.GetPlayerCharacter` 0)))
  (`SceneComponent.SetVisibility` (`/Game/ThirdPersonBP/Blueprints/ThirdPersonCharacter.Bouton E` _asthird_person_character) true false))

(event `self.Box.OnComponentEndOverlap`
  (params (OverlappedComponent :type "PrimitiveComponent Object Reference") (OtherActor :type "Actor Object Reference") (OtherComp :type "PrimitiveComponent Object Reference") (OtherBodyIndex :type Integer))
  (`self.DisableInput` (`GameplayStatics.GetPlayerController` 0))
  (bind _asthird_person_character (cast `/Game/ThirdPersonBP/Blueprints/ThirdPersonCharacter` (`GameplayStatics.GetPlayerCharacter` 0)))
  (`SceneComponent.SetVisibility` (`/Game/ThirdPersonBP/Blueprints/ThirdPersonCharacter.Bouton E` _asthird_person_character) false false))

(fn `UserConstructionScript`
  (bind _returnvalue (`PrimitiveComponent.CreateDynamicMaterialInstance` (`self.Cube(Levier)`) 0 "/Engine/BasicShapes/BasicShapeMaterial.BasicShapeMaterial" "Color"))
  (bind _output_get (set `self.M_DynLevier` _returnvalue))
  (`MaterialInstanceDynamic.SetVectorParameterValue` _output_get "Color" (`self.Couleur`)))