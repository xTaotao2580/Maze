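; Game mode for a 60-second statue-collecting level, running its HUD flow, countdown and score.
; BeginPlay briefly shows a start screen with the GameInstance's high score, then opens the in-game HUD and starts a looping one-second timer.
; CollectStatue adds points and refreshes the HUD; at zero, Timer shows game over and reloads the level.
; Findujeu shows the end screen after a delay, without stopping the timer or saving the score.
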(event `self.ReceiveBeginPlay`
  (bind _ingamehud (`self.InGameHUD`))
  (`|ExecutionSequence`
    (:`then_0`
      ;[1 1 1] Start menu
      (bind _returnvalue (`|CreateWidget` "/Game/UI/DébutHUD.DébutHUD_C"))
      (bind _output_get (set `self.Start HUD` _returnvalue))
      (`UserWidget.AddToViewport` _output_get 0)
      (`|ExecutionSequence`
        (:`then_0`
          (bind _asbp_third_person_game_instance (cast `/Game/Blueprints/BP_ThirdPersonGameInstance` (`GameplayStatics.GetGameInstance`)))
          (`/Game/UI/DébutHUD.HUD High Score` (`self.Start HUD`) (`/Game/Blueprints/BP_ThirdPersonGameInstance.Current High Score` _asbp_third_person_game_instance)))
        (:`then_1`
          (`KismetSystemLibrary.Delay` 3.0)
          (`Widget.RemoveFromParent` (`self.Start HUD`)))))
    (:`then_1`
      ;[1 1 1] In game menu with SCORE, TIME and LEVIERS
      (`KismetSystemLibrary.Delay` 3.0)
      (set `self.Time` 60)
      (bind _returnvalue_2 (`|CreateWidget` "/Game/UI/InGameHUD.InGameHUD_C"))
      (bind _output_get_2 (set `self.InGameHUD` _returnvalue_2))
      (`UserWidget.AddToViewport` _output_get_2 0)
      (`/Game/UI/InGameHUD.Update Score Statue` _ingamehud (`self.Statue count`))
      (`/Game/UI/InGameHUD.Update Timer` _ingamehud (`self.Time`)))
    (:`then_2`
      (`KismetSystemLibrary.Delay` 3.0)
      (`KismetSystemLibrary.K2_SetTimer` null "Timer" 1.0 true))))

(event `Timer`
  ;[1 1 1] Timer countdown with game oevr screen
  (bind _output_get (set `self.Time` (- (`self.Time`) 1)))
  (`/Game/UI/InGameHUD.Update Timer` (`self.InGameHUD`) _output_get)
  (if (== (`self.Time`) 0)
    (`KismetSystemLibrary.K2_ClearTimer` null "Timer")
    (bind _returnvalue (`|CreateWidget` "/Game/UI/GameOverHUD.GameOverHUD_C"))
    (bind _output_get_2 (set `self.GameOver HUD` _returnvalue))
    (`UserWidget.AddToViewport` _output_get_2 0)
    (`KismetSystemLibrary.Delay` 3.0)
    (`Widget.RemoveFromParent` (`self.Start HUD`))
    (bind _returnvalue_2 (`GameplayStatics.GetCurrentLevelName` true))
    (`GameplayStatics.OpenLevel` (`KismetStringLibrary.Conv_StringToName` _returnvalue_2))))

(event `Collect Statue`
  ;[1 1 1] Statue collect = +1000 score
  (`|ExecutionSequence`
    (:`then_0`
      (set `self.Score Statue` (+ (`self.Score Statue`) 1000))
      (`/Game/UI/InGameHUD.Update Score Statue` (`self.InGameHUD`) (`self.Score Statue`)))))

(event `Fin du jeu`
  (`KismetSystemLibrary.Delay` 3.0)
  (bind _returnvalue (`|CreateWidget` "/Game/UI/FinHUD.FinHUD_C"))
  (bind _output_get (set `self.fin HUD` _returnvalue))
  (`UserWidget.AddToViewport` _output_get 0))

(fn `UserConstructionScript`)