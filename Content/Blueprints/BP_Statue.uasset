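; BP_Statue is a collectible pickup that reappears at a random spot each time the player collects it.
; On BeginPlay it caches the BP_ThirdPersonGameMode.
; When the player character overlaps it, it calls CollectStatue on the game mode, destroys itself and spawns a new BP_Statue at a random X/Y within a fixed area at zero height.
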(event `self.ReceiveBeginPlay`
  (bind _asbp_third_person_game_mode (cast `/Game/Blueprints/BP_ThirdPersonGameMode` (`GameplayStatics.GetGameMode`)))
  (set `self.REF_gamemode` _asbp_third_person_game_mode))

(event `self.ReceiveActorBeginOverlap`
  (params (OtherActor :type "Actor Object Reference"))
  ;[1 1 1] Player touch = cast to gamemode, then destroy actor, then actor respawn somewhere random
  (if (== OtherActor (`GameplayStatics.GetPlayerCharacter` 0))
    (`/Game/Blueprints/BP_ThirdPersonGameMode.Collect Statue` (`self.REF_gamemode`))
    (`self.K2_DestroyActor`)
    (`|SpawnActorFromClass` "BP_Statue_C" (`KismetMathLibrary.Conv_VectorToTransform` (`KismetMathLibrary.MakeVector` (`KismetMathLibrary.RandomFloatInRange` -1210.0 400.0) (`KismetMathLibrary.RandomFloatInRange` -1450.0 1325.0))) "Undefined" "OverrideRootScale" null null)))

(fn `UserConstructionScript`)